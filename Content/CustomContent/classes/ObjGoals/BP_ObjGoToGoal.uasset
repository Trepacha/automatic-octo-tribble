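; BP_ObjGoToGoal is a trigger-box actor that completes a "go to" objective when the player reaches it.
; On BeginPlay it caches the player as BP_FirstPersonCharacter.
; When that character overlaps the box while on the matching objective, a one-shot flag is set.
; It then writes the next objective, its type and its required progress directly onto the character, chaining objectives together.
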(event OnComponentBeginOverlap(Box)
  (params (OverlappedComponent :type Primitive%20Component%20Object%20Reference) (OtherActor :type Actor%20Object%20Reference) (OtherComp :type Primitive%20Component%20Object%20Reference) (OtherBodyIndex :type Integer) (bFromSweep :type Boolean) (SweepResult :type Hit%20Result%20Structure%20%28by%20ref%29))
  (bind _char_ref (Variables|Default|GetChar%20REF))
  (if (== OtherActor _char_ref)
    (if (Utilities|Enum|Equal(Enum) (Variables|/Game/FirstPerson/Blueprints/BP_FirstPersonCharacter.BP_FirstPersonCharacter_C|GetCurrent%20Objective _char_ref) (Variables|Default|GetCompletesObjective))
      (if (not (Variables|Default|GetReached))
        (Variables|Default|SetReached true)
        (Variables|/Game/FirstPerson/Blueprints/BP_FirstPersonCharacter.BP_FirstPersonCharacter_C|SetCurrent%20Objective _char_ref (Variables|Default|GetNextObjective))
        (Variables|/Game/FirstPerson/Blueprints/BP_FirstPersonCharacter.BP_FirstPersonCharacter_C|SetObjective%20Type _char_ref (Variables|Default|GetNextObjType))
        (Variables|/Game/FirstPerson/Blueprints/BP_FirstPersonCharacter.BP_FirstPersonCharacter_C|SetObjProgNeeded _char_ref (Variables|Default|GetNextObjProgNeeded))))))

(event EventBeginPlay
  (bind _asbp_first_person_character (Utilities|Casting|CastToBP_FirstPersonCharacter (Game|GetPlayerCharacter 0)))
  (Variables|Default|SetChar%20REF _asbp_first_person_character))

(fn ConstructionScript)