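; BP_ObjCollectGoal is a collectible objective goal that advances the player's current objective when the player overlaps its Box.
; It counts only once, and only if its ForObjective matches the character's CurrentObjective, then increments ObjectiveProgress and optionally destroys itself.
; When progress reaches the needed amount, it resets the count and writes its own next objective, type and required progress onto BP_FirstPersonCharacter, chaining objectives together.
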(event OnComponentBeginOverlap(Box)
  (params (OverlappedComponent :type Primitive%20Component%20Object%20Reference) (OtherActor :type Actor%20Object%20Reference) (OtherComp :type Primitive%20Component%20Object%20Reference) (OtherBodyIndex :type Integer) (bFromSweep :type Boolean) (SweepResult :type Hit%20Result%20Structure%20%28by%20ref%29))
  (if (Utilities|Enum|Equal(Enum) (Variables|Default|GetForObjective) (Variables|/Game/FirstPerson/Blueprints/BP_FirstPersonCharacter.BP_FirstPersonCharacter_C|GetCurrent%20Objective (stale EventBeginPlay _output_get)))
    (if (== OtherActor (stale EventBeginPlay _output_get))
      (if (not (Variables|Default|GetCollected))
        (Variables|/Game/FirstPerson/Blueprints/BP_FirstPersonCharacter.BP_FirstPersonCharacter_C|SetObjective%20Progress (stale EventBeginPlay _output_get) (+ (Variables|/Game/FirstPerson/Blueprints/BP_FirstPersonCharacter.BP_FirstPersonCharacter_C|GetObjective%20Progress (stale EventBeginPlay _output_get)) 1))
        (Variables|Default|SetCollected true)
        (if (Variables|Default|GetShouldActorBeDestroyed)
          (Actor|DestroyActor))
        (if (== (Variables|/Game/FirstPerson/Blueprints/BP_FirstPersonCharacter.BP_FirstPersonCharacter_C|GetObjective%20Progress (stale EventBeginPlay _output_get)) (Variables|/Game/FirstPerson/Blueprints/BP_FirstPersonCharacter.BP_FirstPersonCharacter_C|GetObjProgNeeded (stale EventBeginPlay _output_get)))
          (Variables|/Game/FirstPerson/Blueprints/BP_FirstPersonCharacter.BP_FirstPersonCharacter_C|SetObjective%20Progress (stale EventBeginPlay _output_get) 0)
          (Variables|/Game/FirstPerson/Blueprints/BP_FirstPersonCharacter.BP_FirstPersonCharacter_C|SetCurrent%20Objective (stale EventBeginPlay _output_get) (Variables|Default|GetNextObjective))
          (Variables|/Game/FirstPerson/Blueprints/BP_FirstPersonCharacter.BP_FirstPersonCharacter_C|SetObjective%20Type (stale EventBeginPlay _output_get) (Variables|Default|GetNextObjType))
          (Variables|/Game/FirstPerson/Blueprints/BP_FirstPersonCharacter.BP_FirstPersonCharacter_C|SetObjProgNeeded (Variables|Default|GetChar%20REF) (Variables|Default|GetNextObjProgNeeded)))))))

(event EventBeginPlay
  (bind _asbp_first_person_character (Utilities|Casting|CastToBP_FirstPersonCharacter (Game|GetPlayerCharacter 0)))
  (bind _output_get (Variables|Default|SetChar%20REF _asbp_first_person_character)))

(fn ConstructionScript)