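; BP_Zombie is a zombie enemy pawn that chases the player and dies from point damage.
; On BeginPlay it runs RunToPlayer, an AI MoveTo that targets player controller 0 rather than the player pawn.
; The move re-issues itself only on failure, with no follow-up on success.
; Point damage subtracts from HP and destroys the actor at zero or below.
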(event Custom|Run%20to%20Player
  (AI|AIMoveTo self "0, 0, 0" (Game|GetPlayerController 0) 5.0 false
    (:OnFail
      (CallFunction|RuntoPlayer))))

(event EventBeginPlay
  (CallFunction|RuntoPlayer))

(event Game|Damage|EventPointDamage
  (params (Damage :type Float%20%28single-precision%29) (DamageType :type Damage%20Type%20Object%20Reference) (HitLocation :type Vector :default "0, 0, 0") (HitNormal :type Vector :default "0, 0, 0") (HitComponent :type Primitive%20Component%20Object%20Reference) (BoneName :type Name :default "None") (ShotFromDirection :type Vector :default "0, 0, 0") (InstigatedBy :type Controller%20Object%20Reference) (DamageCauser :type Actor%20Object%20Reference) (HitInfo :type Hit%20Result%20Structure%20%28by%20ref%29))
  (Variables|Default|SetHP (- (Variables|Default|GetHP) Damage))
  (if (<= (Variables|Default|GetHP) 0.0)
    (Actor|DestroyActor)))

(fn ConstructionScript)